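; Door_A_Close_BP is a door actor that reacts to BP_FirstPersonCharacter entering and leaving its overlap, on the actor or component W.
; Begin overlap plays a pressurized door sound and destroys the door instead of animating it.
; End overlap spawns a Door_A_BP at the actor's location, playing the same sound before and after the spawn.
; DoorOpen and DoorClosed record the actor's location but are never read here.
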(event OnComponentBeginOverlap(w)
  (params (OverlappedComponent :type Primitive%20Component%20Object%20Reference) (OtherActor :type Actor%20Object%20Reference) (OtherComp :type Primitive%20Component%20Object%20Reference) (OtherBodyIndex :type Integer) (bFromSweep :type Boolean) (SweepResult :type Hit%20Result%20Structure%20%28by%20ref%29))
  (bind _returnvalue (Transformation|GetActorLocation))
  ;[1 1 1] Open door on begin overlap
  (Utilities|Casting|CastToBP_FirstPersonCharacter OtherActor)
  (Variables|Door|SetDoorOpen _returnvalue)
  (Audio|PlaySoundatLocation "/Game/Audio/AudioSamples/425090__neospica__pressurized-door-opening.425090__neospica__pressurized-door-opening" _returnvalue "0, 0, 0" 1.0 1.0 0.0 0 0 0 0)
  (Actor|DestroyActor))

(event OnComponentEndOverlap(w)
  (params (OverlappedComponent :type Primitive%20Component%20Object%20Reference) (OtherActor :type Actor%20Object%20Reference) (OtherComp :type Primitive%20Component%20Object%20Reference) (OtherBodyIndex :type Integer))
  (bind _returnvalue (Transformation|GetActorLocation))
  (Utilities|Casting|CastToBP_FirstPersonCharacter OtherActor)
  (Variables|Door|SetDoorClosed _returnvalue)
  (Audio|PlaySoundatLocation "/Game/Audio/AudioSamples/425090__neospica__pressurized-door-opening.425090__neospica__pressurized-door-opening" _returnvalue "0, 0, 0" 1.0 1.0 0.0 0 0 0 0)
  (Game|SpawnActorfromClass "/Game/ModSciInteriors/Blueprints/Door_A_BP.Door_A_BP_C" (Math|Conversions|ToTransform(Vector) _returnvalue) "Undefined" 0 0)
  (Audio|PlaySoundatLocation "/Game/Audio/AudioSamples/425090__neospica__pressurized-door-opening.425090__neospica__pressurized-door-opening" _returnvalue "0, 0, 0" 1.0 1.0 0.0 0 0 0 0))

(event EventBeginPlay
  ;[1 1 1] Open door on begin overlap
  (Variables|Door|SetDoorClosed (Transformation|GetActorLocation)))

(event Collision|EventActorBeginOverlap
  (params (OtherActor :type Actor%20Object%20Reference))
  (bind _returnvalue (Transformation|GetActorLocation))
  ;[1 1 1] Open door on begin overlap
  (Utilities|Casting|CastToBP_FirstPersonCharacter (stale OnComponentBeginOverlap(w) OtherActor))
  (Variables|Door|SetDoorOpen _returnvalue)
  (Audio|PlaySoundatLocation "/Game/Audio/AudioSamples/425090__neospica__pressurized-door-opening.425090__neospica__pressurized-door-opening" _returnvalue "0, 0, 0" 1.0 1.0 0.0 0 0 0 0)
  (Actor|DestroyActor))

(event Collision|EventActorEndOverlap
  (params (OtherActor :type Actor%20Object%20Reference))
  (bind _returnvalue (Transformation|GetActorLocation))
  (Utilities|Casting|CastToBP_FirstPersonCharacter (stale OnComponentEndOverlap(w) OtherActor))
  (Variables|Door|SetDoorClosed _returnvalue)
  (Audio|PlaySoundatLocation "/Game/Audio/AudioSamples/425090__neospica__pressurized-door-opening.425090__neospica__pressurized-door-opening" _returnvalue "0, 0, 0" 1.0 1.0 0.0 0 0 0 0)
  (Game|SpawnActorfromClass "/Game/ModSciInteriors/Blueprints/Door_A_BP.Door_A_BP_C" (Math|Conversions|ToTransform(Vector) _returnvalue) "Undefined" 0 0)
  (Audio|PlaySoundatLocation "/Game/Audio/AudioSamples/425090__neospica__pressurized-door-opening.425090__neospica__pressurized-door-opening" _returnvalue "0, 0, 0" 1.0 1.0 0.0 0 0 0 0))

(fn ConstructionScript)